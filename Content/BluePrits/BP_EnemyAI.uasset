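; Melee enemy AI character that chases the player with an axe attack that knocks characters back.
; PawnSensing sightings trigger AI MoveTo toward player 0; on arrival it plays an attack montage, gated by CanAttack until the montage completes or is interrupted.
; A montage notify runs a forward sphere trace, launching any Character hit with forward and upward knockback, plus sound, particles and camera shake, without applying damage.
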(event OnSeePawn(PawnSensing)
  (params (Pawn :type Pawn%20Object%20Reference))
  (CallFunction|ChasePlayer))

(event Custom|Chase%20Player
  (bind _returnvalue (Transformation|GetActorLocation))
  (AI|AIMoveTo self "0, 0, 0" (Game|GetPlayerCharacter 0) 1.2e+02 false
    (:OnSuccess
      (if (Variables|Default|GetcanAttack?)
        (Animation|Montage|PlayMontage (Variables|Character|GetMesh) "/Game/Characters/villager/Animations/Attack/A_Attack_Montage.A_Attack_Montage"
          (:then
            (Variables|Default|SetcanAttack? false)
            (Audio|PlaySoundatLocation "/Game/audio/Sounds/MS_axeHoosh.MS_axeHoosh" (Transformation|GetActorLocation) "0, 0, 0" 1.0 1.0 0.0 0 0 0 0))
          (:OnCompleted
            (Variables|Default|SetcanAttack? true :!label _label))
          (:OnInterrupted
            (goto _label))
          (:OnNotifyBegin
            (bind (_outhit _returnvalue_2) (Collision|SphereTraceByChannel _returnvalue (+ _returnvalue (* (Math|Vector|GetForwardVector (Transformation|GetActorRotation)) 1.8e+02)) 25.0 "TraceTypeQuery3" false 0 "None" true "(R=1.000000,G=0.000000,B=0.000000,A=1.000000)" "(R=0.000000,G=1.000000,B=0.000000,A=1.000000)" 0.5))
            (if _returnvalue_2
              (bind _as角色 (Utilities|Casting|CastToCharacter (.HitActor (Collision|BreakHitResult _outhit))))
              (Character|LaunchCharacter _as角色 (+ (* (Math|Vector|GetForwardVector (Transformation|GetActorRotation)) (Variables|Default|GetFrontalKnckback)) (Math|Vector|MakeVector 0.0 0.0 (Variables|Default|GetUpwardsKnockBack))) false false)
              (Audio|PlaySoundatLocation "/Game/audio/Sounds/MS_axeHit.MS_axeHit" (Transformation|GetActorLocation) "0, 0, 0" 1.0 1.0 0.0 0 0 0 0)
              (Effects|SpawnEmitteratLocation "/Game/Realistic_Starter_VFX_Pack_Vol2/Particles/Hit/P_Wood.P_Wood" (.ImpactPoint (Collision|BreakHitResult _outhit)) (Math|Rotator|MakeRotfromX (.Normal (Collision|BreakHitResult _outhit))) "1.000000,1.000000,1.000000" true "AutoRelease")
              (Camera|PlayWorldCameraShake "/Game/BluePrits/BP_CameraShake_Hit.BP_CameraShake_Hit_C" (.ImpactPoint (Collision|BreakHitResult _outhit)) 0.0 1e+03))))))))

(event EventBeginPlay)

(fn ConstructionScript)